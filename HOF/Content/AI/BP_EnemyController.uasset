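; BP_EnemyController is the AI controller that starts the enemy's behavior tree.
; On BeginPlay it initializes the EnemyBB blackboard with the pawn's starting location as home, an idle time, and a random navigable point around the pawn as the first target location.
; It then runs EnemyBT, with no further logic in Tick or the construction script.
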(event `self.ReceiveBeginPlay`
  (bind _blackboard (`self.Blackboard`))
  (bind _returnvalue (`self.K2_GetActorLocation` (`self.K2_GetPawn`)))
  (`|ExecutionSequence`
    (:`then_0`
      (`self.UseBlackboard` "/Game/AI/EnemyBB.EnemyBB")
      (`BlackboardComponent.SetValueAsVector` _blackboard (`self.HomeLocKey`) _returnvalue)
      (`BlackboardComponent.SetValueAsFloat` _blackboard (`self.IdleTimeKey`) 2.0)
      (`BlackboardComponent.SetValueAsVector` _blackboard (`self.TargetLockey`) (`NavigationSystem.K2_GetRandomLocationInNavigableRadius` _returnvalue 1000.0)))
    (:`then_1`
      (`self.RunBehaviorTree` "/Game/AI/EnemyBT.EnemyBT"))))

(fn `UserConstructionScript`)